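; FireBolt gameplay ability that casts a projectile toward the location under the mouse.
; On activation it gets cursor target data, plays the cast montage and waits for the FireBolt gameplay event.
; That event turns the avatar toward the hit location through CombatInterface, calls SpawnProjectile at that target and ends the ability.
; A leftover delay-then-end branch is unconnected and never runs.
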(event `self.K2_ActivateAbility`
  (bind (_asynctaskproxy _datahandle) (`TargetDataUnderMouse.CreateTargetDataUnderMouse`)
    (:`then`
      (`AbilityTask_PlayMontageAndWait.CreatePlayMontageAndWaitProxy` "None" "/Game/RPG/Characters/Aura/Animations/Abilities/AM_Cast_FireBolt.AM_Cast_FireBolt"
        (:`then`
          (`AbilityTask_WaitGameplayEvent.WaitGameplayEvent` (struct :`TagName` "Event.FireBolt") null
            (:`EventReceived`
              (bind _ascombat_interface (cast `CombatInterface` (`self.GetAvatarActorFromActorInfo`)))
              (bind (_returnvalue_bblockinghit _returnvalue_binitialoverlap _returnvalue_time _returnvalue_distance _returnvalue_location) (`GameplayStatics.BreakHitResult` (`AbilitySystemBlueprintLibrary.GetHitResultFromTargetData` _datahandle)))
              (`CombatInterface.UpdateFacingTarget` _ascombat_interface _returnvalue_location)
              (`self.SpawnProjectile` _returnvalue_location)
              (`self.K2_EndAbility`))))))))